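; Opening cutscene camera that plays a first-person wake-up intro when the game instance's ShouldPlay flag is set.
; On BeginPlay it starts breathing audio, takes over the view and fades a black-screen widget.
; Chained timelines then roll and raise the camera with lerps.
; It finally blends to the player character, enables actions, clears ShouldPlay and opens a dialog with the exit-door task.
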(event `self.ReceiveBeginPlay`
  (if (`/Game/GI_MainGameInstance.ShouldPlay` (cast `/Game/GI_MainGameInstance` (`GameplayStatics.GetGameInstance`) :!pure true))
    (bind _returnvalue (`GameplayStatics.CreateSound2D` "/Game/Sounds/Breathing.Breathing" 1.0 1.0 0.0 null))
    (bind _output_get (set `/Game/GI_MainGameInstance.Music` _returnvalue (cast `/Game/GI_MainGameInstance` (`GameplayStatics.GetGameInstance`) :!pure true)))
    (`AudioComponent.Play` _output_get 0.0)
    (`PlayerController.SetViewTargetWithBlend` (`GameplayStatics.GetPlayerController` 0) self 0.0 "VTBlend_Linear" 0.0 false)
    (bind _returnvalue_2 (`|CreateWidget` "/Game/WB_BlackScreen.WB_BlackScreen_C"))
    (`UserWidget.AddToViewport` _returnvalue_2 0)
    (`SceneComponent.K2_SetRelativeRotation` (`self.Camera`) (`KismetMathLibrary.MakeRotator` (`self.InitialCameraRotationX`)) false false)
    (bind (_direction _rotation1) (`Timeline|Timeline_6`)
      (:`Update`
        (`Widget.SetRenderOpacity` _returnvalue_2 (`KismetMathLibrary.Lerp` 1.0 0.2 _rotation1)))
      (:`Finished`
        (`Widget.RemoveFromParent` _returnvalue_2)
        (bind (_direction_2 _rotation1_2) (`Timeline|Timeline`)
          (:`Update`
            (`SceneComponent.K2_SetRelativeRotation` (`self.Camera`) (`KismetMathLibrary.MakeRotator` (`KismetMathLibrary.Lerp` (`self.InitialCameraRotationX`) 4.0 _rotation1_2)) false false)
            (bind (_direction_3 _rotation1_3) (`Timeline|Timeline_0`)
              (:`Update`
                (`SceneComponent.K2_SetRelativeLocation` (`self.Camera`) (`KismetMathLibrary.MakeVector` 0.0 0.0 (`KismetMathLibrary.Lerp` 0.0 30.0 _rotation1_3)) false false)
                (`KismetSystemLibrary.Delay` 8.0)
                (bind (_direction_4 _rotation1_4) (`Timeline|Timeline_4`)
                  (:`Update`
                    (`SceneComponent.K2_SetRelativeLocation` (`self.Camera`) (`KismetMathLibrary.MakeVector` 0.0 0.0 (`KismetMathLibrary.Lerp` 30.0 90.0 _rotation1_4)) false false)
                    ;[1 1 1] Rotations
                    (bind (_direction_5 _rotation1_5) (`Timeline|Timeline_1`)
                      (:`Update`
                        (`SceneComponent.K2_SetRelativeRotation` (`self.Camera`) (`KismetMathLibrary.MakeRotator` (`KismetMathLibrary.Lerp` 4.0 8.0 _rotation1_5)) false false))
                      (:`Finished`
                        (bind (_direction_6 _rotation1_6) (`Timeline|Timeline_2`)
                          (:`Update`
                            (`SceneComponent.K2_SetRelativeRotation` (`self.Camera`) (`KismetMathLibrary.MakeRotator` (`KismetMathLibrary.Lerp` 8.0 0.0 _rotation1_6)) false false))
                          (:`Finished`
                            (bind _asbp_first_person_character (cast `/Game/FirstPerson/Blueprints/BP_FirstPersonCharacter` (`GameplayStatics.GetPlayerCharacter` 0)))
                            (`PlayerController.SetViewTargetWithBlend` (`GameplayStatics.GetPlayerController` 0) _asbp_first_person_character 1.0 "VTBlend_Linear" 0.0 false)
                            (`KismetSystemLibrary.Delay` 1.0)
                            (set `/Game/GI_MainGameInstance.CanPerformAction` true (cast `/Game/GI_MainGameInstance` (`GameplayStatics.GetGameInstance`) :!pure true))
                            (set `/Game/GI_MainGameInstance.ShouldPlay` false (cast `/Game/GI_MainGameInstance` (`GameplayStatics.GetGameInstance`) :!pure true))
                            (bind _returnvalue_3 (`|CreateWidget` :`Class` "/Game/StoryElements/WB_Dialog.WB_Dialog_C" :`TaskText` "Check the exit door."))
                            (`/Game/StoryElements/WB_Dialog.CreateDialog` _returnvalue_3 (`self.Dialog`) _returnvalue_3 null)
                            (`KismetSystemLibrary.Delay` 2.0)))))))))))))))

(fn `NewFunction`)

(fn `UserConstructionScript`)