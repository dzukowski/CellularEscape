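; End-game trigger actor whose box overlap starts the level completion sequence.
; It crossfades the game instance music to a piano cue and clears the player's active quest text.
; For each timer widget found, it removes and stops it, then blends the view to the endgame camera.
; One timeline slides the camera while creating black-screen widgets; after a delay, another fades in black and finishes with the level-completed window.
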(event `self.Box.OnComponentBeginOverlap`
  (params (OverlappedComponent :type "PrimitiveComponent Object Reference") (OtherActor :type "Actor Object Reference") (OtherComp :type "PrimitiveComponent Object Reference") (OtherBodyIndex :type Integer) (bFromSweep :type Boolean) (SweepResult :type "HitResult Structure (by ref)"))
  (bind _asgi_main_game_instance (cast `/Game/GI_MainGameInstance` (`GameplayStatics.GetGameInstance`) :!pure true))
  (`AudioComponent.FadeOut` (`/Game/GI_MainGameInstance.Music` _asgi_main_game_instance) 2.0 0.0 "Linear")
  (bind _returnvalue (`GameplayStatics.CreateSound2D` "/Game/Sounds/Piano_Cue.Piano_Cue" 1.0 1.0 0.0 null))
  (bind _output_get (set `/Game/GI_MainGameInstance.Music` _returnvalue _asgi_main_game_instance))
  (`AudioComponent.Play` _output_get 0.0)
  (`AudioComponent.FadeIn` _output_get 2.0 1.0 0.0 "Linear")
  (bind _asbp_first_person_character (cast `/Game/FirstPerson/Blueprints/BP_FirstPersonCharacter` (`GameplayStatics.GetPlayerCharacter` 0)))
  (`/Game/WB_ActiveQuest.Update` (`/Game/FirstPerson/Blueprints/BP_FirstPersonCharacter.ActiveQuestWidget` _asbp_first_person_character) "")
  (bind _foundwidgets (`WidgetBlueprintLibrary.GetAllWidgetsOfClass` "/Game/Maze/WB_Timer.WB_Timer_C"))
  (for _array_element _foundwidgets
    (`Widget.RemoveFromParent` _array_element)
    (set `/Game/Maze/WB_Timer.TimerOn` false _array_element)
    (bind _returnvalue_2 (`GameplayStatics.GetActorOfClass` "/Game/BP_EndgameCamera.BP_EndgameCamera_C"))
    (`PlayerController.SetViewTargetWithBlend` (`GameplayStatics.GetPlayerController` 0) _returnvalue_2 1.0 "VTBlend_Linear" 0.0 false)
    (bind (_direction _newtrack_0) (`Timeline|Timeline`)
      (:`Update`
        (`SceneComponent.K2_SetRelativeLocation` (`/Game/BP_EndgameCamera.Camera` _returnvalue_2) (`KismetMathLibrary.MakeVector` (`KismetMathLibrary.Lerp` 0.0 1000.0 _newtrack_0)) false false)
        (bind _returnvalue_3 (`|CreateWidget` "/Game/WB_BlackScreen.WB_BlackScreen_C"))
        (`UserWidget.AddToViewport` _returnvalue_3 0)
        (`Widget.SetRenderOpacity` _returnvalue_3 0.0)
        (`KismetSystemLibrary.Delay` 7.5)
        (bind (_direction_2 _newtrack_0_2) (`Timeline|Timeline_0`)
          (:`Update`
            (`Widget.SetRenderOpacity` _returnvalue_3 (`KismetMathLibrary.Lerp` 0.0 1.0 _newtrack_0_2)))
          (:`Finished`
            (bind _returnvalue_4 (`|CreateWidget` "/Game/WB_LevelCompletedWindow.WB_LevelCompletedWindow_C"))
            (`UserWidget.AddToViewport` _returnvalue_4 0)))))))

(fn `UserConstructionScript`)