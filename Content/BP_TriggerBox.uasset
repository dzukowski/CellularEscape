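; Trigger box actor that fires a door dialog and starts the main level music when its box is overlapped.
; The overlap only acts while the game instance allows the door dialog, then flips its flags so it does not repeat.
; It creates a WB_Dialog with a microscope task text, passes it DialogInfo, and fades in MainLevel_Cue as a 2D sound stored on the game instance.
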(event `self.Box.OnComponentBeginOverlap`
  (params (OverlappedComponent :type "PrimitiveComponent Object Reference") (OtherActor :type "Actor Object Reference") (OtherComp :type "PrimitiveComponent Object Reference") (OtherBodyIndex :type Integer) (bFromSweep :type Boolean) (SweepResult :type "HitResult Structure (by ref)"))
  (if (`/Game/GI_MainGameInstance.CanActivateDoorDialog` (cast `/Game/GI_MainGameInstance` (`GameplayStatics.GetGameInstance`) :!pure true))
    (set `/Game/GI_MainGameInstance.WasDoorDialogActivated` true (cast `/Game/GI_MainGameInstance` (`GameplayStatics.GetGameInstance`) :!pure true))
    (bind _returnvalue (`|CreateWidget` :`Class` "/Game/StoryElements/WB_Dialog.WB_Dialog_C" :`TaskText` "Use the microscope."))
    (`/Game/StoryElements/WB_Dialog.CreateDialog` _returnvalue (`self.Dialog Info`) _returnvalue null)
    (set `/Game/GI_MainGameInstance.CanActivateDoorDialog` false (cast `/Game/GI_MainGameInstance` (`GameplayStatics.GetGameInstance`) :!pure true))
    (bind _asgi_main_game_instance (cast `/Game/GI_MainGameInstance` (`GameplayStatics.GetGameInstance`)))
    (bind _returnvalue_2 (`GameplayStatics.CreateSound2D` "/Game/Sounds/MainLevel_Cue.MainLevel_Cue" 1.0 1.0 0.0 null))
    (bind _output_get (set `/Game/GI_MainGameInstance.Music` _returnvalue_2 _asgi_main_game_instance))
    (`AudioComponent.Play` _output_get 0.0)
    (`AudioComponent.FadeIn` _output_get 3.0 1.0 0.0 "Linear")))

(fn `UserConstructionScript`)