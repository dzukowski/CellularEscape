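; BP_AccessPad is an access pad that opens the level's BP_Door once the space shooter is complete.
; Its box overlap toggles input and, if the door dialog was activated and the door is closed, shows an action prompt widget.
; Pressing E checks GI_MainGameInstance flags, then either plays a granted sound and calls OpenDoor, or plays a denied sound.
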(event `self.Box.OnComponentBeginOverlap`
  (params (OverlappedComponent :type "PrimitiveComponent Object Reference") (OtherActor :type "Actor Object Reference") (OtherComp :type "PrimitiveComponent Object Reference") (OtherBodyIndex :type Integer) (bFromSweep :type Boolean) (SweepResult :type "HitResult Structure (by ref)"))
  (`self.EnableInput` (`GameplayStatics.GetPlayerController` 0))
  (if (`/Game/GI_MainGameInstance.WasDoorDialogActivated` (cast `/Game/GI_MainGameInstance` (`GameplayStatics.GetGameInstance`) :!pure true))
    (if (not (`/Game/GI_MainGameInstance.IsDoorOpen` (cast `/Game/GI_MainGameInstance` (`GameplayStatics.GetGameInstance`) :!pure true)))
      (bind _returnvalue (`|CreateWidget` "/Game/WB_ActionDescription.WB_ActionDescription_C" null "to open the door"))
      (`UserWidget.AddToViewport` _returnvalue 0))))

(event `self.Box.OnComponentEndOverlap`
  (params (OverlappedComponent :type "PrimitiveComponent Object Reference") (OtherActor :type "Actor Object Reference") (OtherComp :type "PrimitiveComponent Object Reference") (OtherBodyIndex :type Integer))
  (`self.DisableInput` (`GameplayStatics.GetPlayerController` 0))
  (if (`/Game/GI_MainGameInstance.WasDoorDialogActivated` (cast `/Game/GI_MainGameInstance` (`GameplayStatics.GetGameInstance`) :!pure true))
    (`Widget.RemoveFromParent` (stale `self.Box.OnComponentBeginOverlap` _returnvalue))))

(event `Key|E` :consume false
  (params (Key :type "Key Structure"))
  (:`Pressed`
    (bind _asgi_main_game_instance (cast `/Game/GI_MainGameInstance` (`GameplayStatics.GetGameInstance`)))
    (if (`/Game/GI_MainGameInstance.IsDoorOpen` _asgi_main_game_instance)
      _
      (elif (`/Game/GI_MainGameInstance.IsSpaceShooterComplete` _asgi_main_game_instance)
        (`GameplayStatics.PlaySound2D` "/Game/Sounds/AccessGranted.AccessGranted" 1.5 1.0 0.0 null null)
        (bind _returnvalue (`GameplayStatics.GetActorOfClass` "/Game/Door/BP_Door.BP_Door_C"))
        (`/Game/Door/BP_Door.OpenDoor` _returnvalue)
        (else
          (`GameplayStatics.PlaySound2D` "/Game/Sounds/AccessDenied2.AccessDenied2" 1.5 1.0 0.0 null null))))))

(fn `UserConstructionScript`)