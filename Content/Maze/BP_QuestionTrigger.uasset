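; BP_QuestionTrigger is a maze trigger volume that shows a timed question to the player on overlap.
; On Box overlap it hides its TextRender and, if no widget is active, creates a WB_Question with its QuestionContent and adds it to the viewport.
; After a five-second delay it removes and clears the widget, then shows the text again.
; The overlap does not filter which actor entered.
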(event `self.ReceiveBeginPlay`)

(event `self.Box.OnComponentBeginOverlap`
  (params (OverlappedComponent :type "PrimitiveComponent Object Reference") (OtherActor :type "Actor Object Reference") (OtherComp :type "PrimitiveComponent Object Reference") (OtherBodyIndex :type Integer) (bFromSweep :type Boolean) (SweepResult :type "HitResult Structure (by ref)"))
  (`SceneComponent.SetHiddenInGame` (`self.TextRender`) true false)
  (`/Engine/EditorBlueprintResources/StandardMacros.IsValid` (`self.WidgetReference`)
    (:`Is Not Valid`
      (bind _returnvalue (`|CreateWidget` "/Game/Maze/WB_Question.WB_Question_C" null (`self.Question Content`)))
      (bind _output_get (set `self.WidgetReference` _returnvalue))
      (`UserWidget.AddToViewport` _output_get 0)
      (`KismetSystemLibrary.Delay` 5.0)
      (`Widget.RemoveFromParent` _output_get)
      (set `self.WidgetReference` null)
      (`SceneComponent.SetHiddenInGame` (`self.TextRender`) false false))))

(fn `UserConstructionScript`)