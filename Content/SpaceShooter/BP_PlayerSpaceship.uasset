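; BP_PlayerSpaceship is the player ship in the space shooter, moving along world X and firing projectiles.
; BeginPlay switches the view to BP_FixedCamera, positions the ship at half the viewport width and creates the HUD.
; The Move axis drives movement input, then clamps X around the start position using viewport pixel width as world units, refreshed on Tick.
; SpaceBar spawns BP_Projectile, gated by a one-second CanShoot cooldown.
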(event `self.ReceiveBeginPlay`
  (bind _returnvalue_x (`KismetMathLibrary.BreakVector` (`self.K2_GetActorLocation`)))
  (bind _returnvalue_x_2 (`KismetMathLibrary.BreakVector2D` (`WidgetLayoutLibrary.GetViewportSize`)))
  (bind (_returnvalue_x_3 _returnvalue_y _returnvalue_z) (`KismetMathLibrary.BreakVector` (`self.K2_GetActorLocation`)))
  (bind _returnvalue_x_4 (`KismetMathLibrary.BreakVector` (`self.K2_GetActorLocation`)))
  (bind _screenlocation (`PlayerController.ProjectWorldLocationToScreen` (`GameplayStatics.GetPlayerController` 0) (`KismetMathLibrary.MakeVector` _returnvalue_x_4) false))
  (bind _returnvalue (`GameplayStatics.GetActorOfClass` "/Game/SpaceShooter/BP_FixedCamera.BP_FixedCamera_C"))
  (`PlayerController.SetViewTargetWithBlend` (`GameplayStatics.GetPlayerController` 0) _returnvalue 0.0 "VTBlend_Linear" 0.0 false)
  (`self.K2_SetActorLocation` (`KismetMathLibrary.MakeVector` (/ _returnvalue_x_2 2.0) _returnvalue_y _returnvalue_z))
  (set `self.Return Value X` _returnvalue_x)
  (set `self.StartingLocation` (`self.K2_GetActorLocation`))
  (set `self.Screen Location X` (`KismetMathLibrary.BreakVector2D` _screenlocation))
  (set `self.SpaceshipHalfWidth` (/ (`KismetMathLibrary.Abs` (- (`KismetMathLibrary.BreakVector2D` _screenlocation) (`KismetMathLibrary.BreakVector2D` (`PlayerController.ProjectWorldLocationToScreen` (`GameplayStatics.GetPlayerController` 0) (`KismetMathLibrary.MakeVector` (.x (`.BoxExtent` (`self.GetActorBounds` false)))) false)))) 2.0))
  (bind _returnvalue_2 (`|CreateWidget` "/Game/SpaceShooter/UI/WB_SpaceShooterHUD.WB_SpaceShooterHUD_C"))
  (bind _output_get (set `self.SpaceShooterHUD` _returnvalue_2))
  (`UserWidget.AddToViewport` _output_get 0))

(event `self.ReceiveTick`
  (params (DeltaSeconds :type "Float (single-precision)"))
  (bind _returnvalue_x (`KismetMathLibrary.BreakVector2D` (`WidgetLayoutLibrary.GetViewportSize`)))
  (set `self.ViewportWidth` _returnvalue_x))

(event `InputAxis|Move`
  (params (AxisValue :type "Float (single-precision)"))
  (bind (_returnvalue_x _returnvalue_y _returnvalue_z) (`KismetMathLibrary.BreakVector` (`self.K2_GetActorLocation`)))
  (bind _returnvalue (/ (`self.ViewportWidth`) 2.0))
  (`self.AddMovementInput` (1.0 0.0 0.0) AxisValue)
  (`self.K2_SetActorLocation` (`KismetMathLibrary.MakeVector` (`KismetMathLibrary.FClamp` _returnvalue_x (+ (- (`self.Return Value X`) _returnvalue) 150.0) (- (+ (`self.Return Value X`) _returnvalue) 50.0)) _returnvalue_y _returnvalue_z)))

(event `Key|SpaceBar`
  (params (Key :type "Key Structure"))
  (:`Pressed`
    (if (`self.CanShoot`)
      (set `self.CanShoot` false)
      (`|SpawnActorFromClass` "/Game/SpaceShooter/BP_Projectile.BP_Projectile_C" (`KismetMathLibrary.MakeTransform` (`SceneComponent.GetSocketLocation` (`self.Scene`) "None") (struct :`Yaw` 90.0)) "Undefined" "MultiplyWithRoot" null null)
      (`KismetSystemLibrary.Delay` 1.0)
      (set `self.CanShoot` true))))

(fn `UserConstructionScript`)