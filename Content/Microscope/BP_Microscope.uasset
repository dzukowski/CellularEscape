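; Interactable microscope actor that opens a cell-observation widget once the game instance's door dialog flag is set.
; Box overlap tracks range, toggles an action prompt and enables the mesh's custom depth, which end overlap also sets true rather than clearing.
; The EEE input in range pauses the game and shows a proceed-question widget.
; Its OnProceed event records microscope activation in the game instance and opens the microscope widget.
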(event `self.ReceiveBeginPlay`
  (`self.EnableInput` (`GameplayStatics.GetPlayerController` 0)))

(event `InputAction|Input EEE` :consume false
  (params (Key :type "Key Structure"))
  (:`Pressed`
    (if (`/Game/GI_MainGameInstance.WasDoorDialogActivated` (cast `/Game/GI_MainGameInstance` (`GameplayStatics.GetGameInstance`) :!pure true))
      (if (`self.IsOverlapping`)
        (bind _returnvalue (`|CreateWidget` "/Game/UI/WB_ProceedQuestion.WB_ProceedQuestion_C"))
        (`UserWidget.AddToViewport` _returnvalue 0)
        (set `PlayerController.bShowMouseCursor` true (`GameplayStatics.GetPlayerController` 0))
        (`GameplayStatics.SetGamePaused` true)
        (add `/Game/UI/WB_ProceedQuestion.OnProceed` _returnvalue (delegate `Proceed`))))))

(event `Proceed`
  (set `/Game/GI_MainGameInstance.WasMicroscopeActivated` true (cast `/Game/GI_MainGameInstance` (`GameplayStatics.GetGameInstance`) :!pure true))
  (bind _returnvalue (`|CreateWidget` "/Game/Microscope/WB_Microscope.WB_Microscope_C"))
  (`UserWidget.AddToViewport` _returnvalue 0))

(event `self.Box.OnComponentBeginOverlap`
  (params (OverlappedComponent :type "PrimitiveComponent Object Reference") (OtherActor :type "Actor Object Reference") (OtherComp :type "PrimitiveComponent Object Reference") (OtherBodyIndex :type Integer) (bFromSweep :type Boolean) (SweepResult :type "HitResult Structure (by ref)"))
  (set `self.IsOverlapping` true)
  (`PrimitiveComponent.SetRenderCustomDepth` (`self.StaticMesh`) true)
  (if (`/Game/GI_MainGameInstance.WasDoorDialogActivated` (cast `/Game/GI_MainGameInstance` (`GameplayStatics.GetGameInstance`) :!pure true))
    (bind _returnvalue (`|CreateWidget` "/Game/WB_ActionDescription.WB_ActionDescription_C" null "to observe cells under the microscope"))
    (`UserWidget.AddToViewport` _returnvalue 0)))

(event `self.Box.OnComponentEndOverlap`
  (params (OverlappedComponent :type "PrimitiveComponent Object Reference") (OtherActor :type "Actor Object Reference") (OtherComp :type "PrimitiveComponent Object Reference") (OtherBodyIndex :type Integer))
  (`PrimitiveComponent.SetRenderCustomDepth` (`self.StaticMesh`) true)
  (set `self.IsOverlapping` false)
  (if (`/Game/GI_MainGameInstance.WasDoorDialogActivated` (cast `/Game/GI_MainGameInstance` (`GameplayStatics.GetGameInstance`) :!pure true))
    (`Widget.RemoveFromParent` (stale `self.Box.OnComponentBeginOverlap` _returnvalue))))

(fn `UserConstructionScript`)