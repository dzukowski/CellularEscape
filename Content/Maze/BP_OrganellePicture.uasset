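; BP_OrganellePicture is a maze pickup showing an organelle picture and name, both set per instance in the construction script from a material and text variable.
; Overlapping its box once hides the actor.
; A correct picture plays a sound, while a wrong one moves the player to a fixed location, likely sending them back in the maze.
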(event `self.BoxCollision.OnComponentBeginOverlap`
  (params (OverlappedComponent :type "PrimitiveComponent Object Reference") (OtherActor :type "Actor Object Reference") (OtherComp :type "PrimitiveComponent Object Reference") (OtherBodyIndex :type Integer) (bFromSweep :type Boolean) (SweepResult :type "HitResult Structure (by ref)"))
  (if (`self.CanTrigger`)
    (`self.SetActorHiddenInGame` true)
    (if (`self.IsCorrect`)
      (`GameplayStatics.PlaySound2D` "/Game/Sounds/Correct.Correct" 1.0 1.0 0.0 null null)
      (else
        (`self.K2_SetActorLocation` (`GameplayStatics.GetPlayerCharacter` 0) (739.087809 922.63725 144.088314) false false)))
    (set `self.CanTrigger` false)))

(fn `UserConstructionScript`
  (`PrimitiveComponent.SetMaterial` (`self.Picture`) 0 (`self.Material`))
  (`TextRenderComponent.K2_SetText` (`self.TextRender`) (`self.OrganelleName`)))