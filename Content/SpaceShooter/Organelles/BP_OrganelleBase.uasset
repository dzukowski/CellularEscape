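; BP_OrganelleBase is the base actor for shootable organelle targets in the space shooter minigame.
; Its construction script applies a configurable mesh and sets a text label to the organelle's name.
; When a BP_Projectile hits its box, it compares CellType to ChosenCellType and updates either the correct score or the mistakes on the player ship's HUD, then destroys itself.
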(event `self.ReceiveBeginPlay`)

(event `self.Box.OnComponentHit`
  (params (HitComponent :type "PrimitiveComponent Object Reference") (OtherActor :type "Actor Object Reference") (OtherComp :type "PrimitiveComponent Object Reference") (NormalImpulse :type "Vector Structure") (Hit :type "HitResult Structure (by ref)"))
  (bind _spaceshooterhud (`/Game/SpaceShooter/BP_PlayerSpaceship.SpaceShooterHUD` (cast `/Game/SpaceShooter/BP_PlayerSpaceship` (`GameplayStatics.GetPlayerPawn` 0) :!pure true)))
  (cast `/Game/SpaceShooter/BP_Projectile` OtherActor)
  (if (`|EnumEquality` (`self.CellType`) (`self.ChosenCellType`))
    (`/Game/SpaceShooter/UI/WB_SpaceShooterHUD.UpdateCorrectScore` _spaceshooterhud)
    (else
      (`/Game/SpaceShooter/UI/WB_SpaceShooterHUD.UpdateMistakes` _spaceshooterhud)))
  (`self.K2_DestroyActor`))

(fn `UserConstructionScript`
  (`StaticMeshComponent.SetStaticMesh` (`self.Model`) (`self.New Mesh`))
  (`TextRenderComponent.K2_SetText` (`self.TextRender`) (`self.Name`)))