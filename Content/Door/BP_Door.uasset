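; BP_Door is a double sliding door actor that opens through its OpenDoor event and records that state in the game instance.
; OpenDoor clears the player character's active quest widget with an empty update, then plays the Open timeline.
; Each timeline update slides RDoor and LDoor apart along relative X and sets IsDoorOpen on GI_MainGameInstance.
; BeginPlay enables player input on the actor, though no input events are defined here.
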(event `self.ReceiveBeginPlay`
  (`self.EnableInput` (`GameplayStatics.GetPlayerController` 0)))

(event `OpenDoor`
  (bind _asbp_first_person_character (cast `/Game/FirstPerson/Blueprints/BP_FirstPersonCharacter` (`GameplayStatics.GetPlayerCharacter` 0)))
  (`/Game/WB_ActiveQuest.Update` (`/Game/FirstPerson/Blueprints/BP_FirstPersonCharacter.ActiveQuestWidget` _asbp_first_person_character) "")
  (bind (_direction _newtrack_0) (`Timeline|Open`)
    (:`Update`
      (`SceneComponent.K2_SetRelativeLocation` (`self.R_Door`) (`KismetMathLibrary.MakeVector` (`KismetMathLibrary.Lerp` 0.0 100.0 _newtrack_0)) false false)
      (`SceneComponent.K2_SetRelativeLocation` (`self.L_Door`) (`KismetMathLibrary.MakeVector` (`KismetMathLibrary.Lerp` 0.0 -100.0 _newtrack_0)) false false)
      (bind _asgi_main_game_instance (cast `/Game/GI_MainGameInstance` (`GameplayStatics.GetGameInstance`)))
      (set `/Game/GI_MainGameInstance.IsDoorOpen` true _asgi_main_game_instance))))

(fn `UserConstructionScript`)