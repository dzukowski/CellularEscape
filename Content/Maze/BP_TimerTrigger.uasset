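; BP_TimerTrigger is a maze trigger that puts the timer on screen and switches the music when its Box is overlapped.
; If TimerReference is not valid, the overlap creates a WB_Timer widget, stores it and adds it to the viewport.
; In the same branch it stops the Music held by GI_MainGameInstance, then replaces and plays it with MazeMusic1.
; The overlapping actor is not filtered.
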(event `self.Box.OnComponentBeginOverlap`
  (params (OverlappedComponent :type "PrimitiveComponent Object Reference") (OtherActor :type "Actor Object Reference") (OtherComp :type "PrimitiveComponent Object Reference") (OtherBodyIndex :type Integer) (bFromSweep :type Boolean) (SweepResult :type "HitResult Structure (by ref)"))
  (`/Engine/EditorBlueprintResources/StandardMacros.IsValid` (`self.TimerReference`)
    (:`Is Not Valid`
      (bind _returnvalue (`|CreateWidget` "/Game/Maze/WB_Timer.WB_Timer_C"))
      (bind _output_get (set `self.TimerReference` _returnvalue))
      (`UserWidget.AddToViewport` _output_get 0)
      (`AudioComponent.Stop` (`/Game/GI_MainGameInstance.Music` (cast `/Game/GI_MainGameInstance` (`GameplayStatics.GetGameInstance`) :!pure true)))
      (bind _returnvalue_2 (`GameplayStatics.CreateSound2D` "/Game/Sounds/MazeMusic1.MazeMusic1" 1.0 1.0 0.0 null))
      (bind _output_get_2 (set `/Game/GI_MainGameInstance.Music` _returnvalue_2 (cast `/Game/GI_MainGameInstance` (`GameplayStatics.GetGameInstance`) :!pure true)))
      (`AudioComponent.Play` _output_get_2 0.0))))

(fn `UserConstructionScript`)